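; Base player pawn Blueprint with click-to-move navigation and a visible mouse cursor.
; BeginPlay adds either the WASD or click-to-move Enhanced Input mapping context according to the control mode.
; IA_Move line-traces under the cursor on Visibility, with debug drawing, and passes the hit location to SimpleMoveToLocation.
; Tick rotates the actor toward a MousePosition variable, which these graphs never set.
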(event `EnhancedInput|/Game/Core/Blueprints/ControlSystem/Actions/CTM/IA_Move`
  (params (ActionValue :type Boolean) (ElapsedSeconds :type "Float (double-precision)") (TriggeredSeconds :type "Float (double-precision)") (InputAction :type "InputAction Object Reference" :default "/Game/Core/Blueprints/ControlSystem/Actions/CTM/IA_Move.IA_Move"))
  ;[0.2984 0.3699 0.599] Input Events
  (:`Triggered`
    (`self.Click To Move`)))

(event `self.ReceiveBeginPlay`
  ;[0.2794 0.7855 0.9635] Main Events
  (`self.Initialize Mapping Context` (`self.Control-mode`))
  (`self.ShowCursor`))

(event `self.ReceiveTick`
  (params (DeltaSeconds :type "Float (single-precision)"))
  ;[0.2794 0.7855 0.9635] Main Events
  (`self.K2_SetActorRotation` (`KismetMathLibrary.FindLookAtRotation` (`self.K2_GetActorLocation`) (`self.MousePosition`))))

(fn `Click To Move`
  (returns (MovingPosition :type "Vector Structure"))
  (bind _outhit (`self.Get Target Position`))
  (bind (_bblockinghit _binitialoverlap _time _distance _location) (`GameplayStatics.BreakHitResult` _outhit))
  (`AIBlueprintHelperLibrary.SimpleMoveToLocation` (`GameplayStatics.GetPlayerController` 0) _location)
  (return _location))

(fn `Get Target Position`
  (returns (OutHit :type "HitResult Structure"))
  (bind (_worldlocation _worlddirection) (`PlayerController.DeprojectMousePositionToWorld` (`GameplayStatics.GetPlayerController` 0)))
  (bind _outhit (`KismetSystemLibrary.LineTraceSingle` :`Start` _worldlocation :`End` (+ _worldlocation (* _worlddirection 5000)) :`TraceChannel` "TraceTypeQuery1" :`DrawDebugType` "ForDuration"))
  (return _outhit))

(fn `Initialize Mapping Context`
  (params (`Control-Mode` :type "/Game/Core/Blueprints/ControlSystem/ENUM_Control-Type Enum" :default "NewEnumerator0"))
  (bind _asplayer_controller (cast `PlayerController` (`self.GetController`)))
  (bind _returnvalue (pcsubsystem `EnhancedInputLocalPlayerSubsystem` _asplayer_controller))
  (`/Engine/EditorBlueprintResources/StandardMacros.IsValid` _returnvalue
    (:`Is Valid`
      (switch `/Game/Core/Blueprints/ControlSystem/ENUM_Control-Type` `Control-Mode`
        (:`NewEnumerator0`
          (`EnhancedInputSubsystemInterface.AddMappingContext` _returnvalue "/Game/Core/Blueprints/ControlSystem/WASD_Mapping.WASD_Mapping" 0 (struct)))
        (:`NewEnumerator1`
          (`EnhancedInputSubsystemInterface.AddMappingContext` _returnvalue "/Game/Core/Blueprints/ControlSystem/CTM_Mapping.CTM_Mapping" 0 (struct)))))))

(fn `ShowCursor`
  (set `PlayerController.bShowMouseCursor` true (`GameplayStatics.GetPlayerController` 0)))

(fn `UserConstructionScript`)