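; Player pawn Blueprint for mouse click-to-move, which adds the WASD_Controls Enhanced Input mapping context and shows the cursor on BeginPlay.
; IA_ClickToMove is meant to trigger a routine that deprojects the cursor and line-traces 500 units on the Visibility channel.
; That routine passes the hit location to SimpleMoveToLocation without checking for a hit, printing debug values along the way.
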(event `self.ReceiveBeginPlay`
  (bind _asplayer_controller (cast `PlayerController` (`self.GetController`)))
  (bind _returnvalue (pcsubsystem `EnhancedInputLocalPlayerSubsystem` _asplayer_controller))
  (`/Engine/EditorBlueprintResources/StandardMacros.IsValid` _returnvalue
    (:`Is Valid`
      (`EnhancedInputSubsystemInterface.AddMappingContext` _returnvalue "/Game/Core/WASD_Controls.WASD_Controls" 0 (struct))
      (`self.ShowMouseCursor`))))

(event `ShowMouseCursor`
  (set `PlayerController.bShowMouseCursor` true (`GameplayStatics.GetPlayerController` 0)))

(event `Player_Controller`
  (bind (_worldlocation _worlddirection) (`PlayerController.DeprojectMousePositionToWorld` (`GameplayStatics.GetPlayerController` 0)))
  (bind _returnvalue (+ _worldlocation (* _worlddirection 500)))
  (`KismetSystemLibrary.PrintString` (`KismetStringLibrary.Conv_VectorToString` _returnvalue))
  (bind (_outhit _returnvalue_2) (`KismetSystemLibrary.LineTraceSingle` _worldlocation _returnvalue "TraceTypeQuery1"))
  (`KismetSystemLibrary.PrintString` (`KismetStringLibrary.Conv_BoolToString` _returnvalue_2))
  (`AIBlueprintHelperLibrary.SimpleMoveToLocation` (`GameplayStatics.GetPlayerController` 0) (`.Location` (`GameplayStatics.BreakHitResult` _outhit))))

(event `EnhancedInput|/Game/Core/Action/IA_ClickToMove`
  (params (ActionValue :type Boolean) (ElapsedSeconds :type "Float (double-precision)") (TriggeredSeconds :type "Float (double-precision)") (InputAction :type "InputAction Object Reference" :default "/Game/Core/Action/IA_ClickToMove.IA_ClickToMove"))
  (:`Started`
    (`KismetSystemLibrary.PrintString` "Pressed")
    (`self.Player_Controller`)))

(fn `UserConstructionScript`)